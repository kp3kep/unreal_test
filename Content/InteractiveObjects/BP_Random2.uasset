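; BP_Random2 is an interactive sphere object whose color and uniform scale can be changed at runtime and read back.
; On BeginPlay it swaps in a dynamic material instance on the Sphere and caches the starting Color parameter and X scale.
; UpdateColor and UpdateScale events apply new values to the material and mesh while storing them for the GetColor and GetScale functions.
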(event EventBeginPlay
  (bind _sphere (Variables|Default|GetSphere))
  (bind _returnvalue (Rendering|Material|CreateDynamicMaterialInstance (Rendering|Material|GetMaterial _sphere 0) "None" "None" :!class /Script/Engine.KismetMaterialLibrary))
  (bind _output_get (Variables|Default|SetMaterialInstance _returnvalue))
  (Rendering|Material|SetMaterial _sphere 0 _output_get)
  (bind _returnvalue_2 (Rendering|Material|GetVectorParameterValue _output_get "Color" :!class /Script/Engine.MaterialInstanceDynamic))
  (Variables|Default|SetColor _returnvalue_2)
  (Variables|Default|SetScale (.x (Variables|/Script/Engine.SceneComponent|GetRelativeScale3D (Variables|Default|GetSphere)))))

(event EventUpdateColor
  (params (InColor :type Linear%20Color%20Structure%20%28by%20ref%29))
  (bind _output_get (Variables|Default|SetColor InColor))
  (Rendering|Material|SetVectorParameterValue (Variables|Default|GetMaterialInstance) "Color" _output_get :!class /Script/Engine.MaterialInstanceDynamic))

(event EventUpdateScale
  (params (InScale :type Float%20%28single-precision%29))
  (bind _output_get (Variables|Default|SetScale InScale))
  (Transformation|SetRelativeScale3D (Variables|Default|GetSphere) (Math|Conversions|ToVector(Float) _output_get)))

(fn ConstructionScript)

(fn GetColor
  (return (Variables|Default|GetColor)))

(fn GetScale
  (return (Variables|Default|GetScale)))