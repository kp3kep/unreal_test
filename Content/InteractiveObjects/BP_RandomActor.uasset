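; BP_RandomActor is an interactive cube actor whose color and uniform scale can be read and changed through an Interactive Object interface.
; On BeginPlay it puts a dynamic material instance on the cube, then caches the initial BaseColor and X scale as its Color and Scale.
; UpdateColor and UpdateScale store new values and apply them to the material and mesh, while GetColor and GetScale return the cached state.
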(event EventBeginPlay
  (CallFunction|CreateMaterialInstance)
  (CallFunction|InitializeLocalColorandScale))

(event EventUpdateScale
  (params (InScale :type Float%20%28single-precision%29))
  ;[0.15 0.15 0.15 0.5] Interactive Object Interface
  (bind _output_get (Variables|Default|SetScale InScale))
  (Transformation|SetRelativeScale3D (Variables|Default|GetCube) (Math|Conversions|ToVector(Float) _output_get)))

(event EventUpdateColor
  (params (InColor :type Linear%20Color%20Structure%20%28by%20ref%29))
  ;[0.15 0.15 0.15 0.5] Interactive Object Interface
  (bind _output_get (Variables|Default|SetColor InColor))
  (Rendering|Material|SetVectorParameterValue (Variables|Default|GetMaterialInstance) "BaseColor" _output_get :!class /Script/Engine.MaterialInstanceDynamic))

(fn ConstructionScript)

(fn CreateMaterialInstance
  (bind _returnvalue (Rendering|Material|CreateDynamicMaterialInstance (Rendering|Material|GetMaterial (Variables|Default|GetCube) 0) "None" "None" :!class /Script/Engine.KismetMaterialLibrary))
  (bind _output_get (Variables|Default|SetMaterialInstance _returnvalue))
  (Rendering|Material|SetMaterial (Variables|Default|GetCube) 0 _output_get)
  (return))

(fn InitializeLocalColorandScale
  (bind _returnvalue (Rendering|Material|GetVectorParameterValue (Variables|Default|GetMaterialInstance) "BaseColor" :!class /Script/Engine.MaterialInstanceDynamic))
  (Variables|Default|SetColor _returnvalue)
  (Variables|Default|SetScale (.x (Variables|/Script/Engine.SceneComponent|GetRelativeScale3D (Variables|Default|GetCube)))))

(fn GetColor
  (return (Variables|Default|GetColor)))

(fn GetScale
  (return (Variables|Default|GetScale)))